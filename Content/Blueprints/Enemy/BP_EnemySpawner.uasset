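; Enemy spawner that periodically spawns BP_Enemy actors near the player character.
; On BeginPlay it starts a looping timer that calls Spawn at the SpawnTimer interval.
; Spawn offsets player 0's location by independent random X and Y values, each between MinDistance and MaxDistance, with no vertical offset.
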(event EventBeginPlay
  (Utilities|Time|SetTimerbyFunctionName 0 "Spawn" (Variables|Spawner|GetSpawn%20Timer) true))

(fn ConstructionScript)

(fn Spawn
  (Game|SpawnActorfromClass "/Game/Blueprints/Enemy/BP_Enemy.BP_Enemy_C" (Math|Transform|MakeTransform (+ (Transformation|GetActorLocation (Game|GetPlayerCharacter 0)) (Math|Vector|MakeVector (Math|Random|RandomFloatinRange (Variables|Spawner|GetMin%20Distance) (Variables|Spawner|GetMax%20Distance)) (Math|Random|RandomFloatinRange (Variables|Spawner|GetMin%20Distance) (Variables|Spawner|GetMax%20Distance)) 0.0)) "0, 0, 0" "1.000000,1.000000,1.000000") "Undefined" "MultiplyWithRoot" 0 0))