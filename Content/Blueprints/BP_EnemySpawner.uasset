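; Enemy spawner that periodically spawns enemies at random points around the BP_IronSoul player character.
; On BeginPlay it stores an existing BP_Enemy from the level, whose class it spawns, and starts a looping Spawn timer.
; Each spawn offsets the player's location by a flattened, unnormalized random vector scaled between MinDistance and MaxDistance, so enemies can land inside the minimum.
; A debug print re-rolls that random position, so it can differ from the actual spawn point.
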(event EventBeginPlay
  (bind _returnvalue (Actor|GetActorOfClass "/Game/Blueprints/Enemy/BP_Enemy.BP_Enemy_C"))
  (Variables|Default|SetEnemies _returnvalue)
  (Utilities|Time|SetTimerbyFunctionName 0 "Spawn" (Variables|Spawner|GetSpawn%20Timer) true))

(fn ConstructionScript)

(fn Spawn
  (bind _returnvalue (Math|Random|RandomUnitVector))
  (bind _asbp_iron_soul (Utilities|Casting|CastToBP_IronSoul (Game|GetPlayerCharacter 0)))
  (Development|PrintString (Utilities|String|ToString(Vector) (+ (Transformation|GetActorLocation _asbp_iron_soul) (* (Math|Vector|MakeVector (.x _returnvalue) (.y _returnvalue) 0.0) (Math|Random|RandomFloatinRange (Variables|Spawner|GetMin%20Distance) (Variables|Spawner|GetMax%20Distance))))) true true "(R=0.000000,G=0.660000,B=1.000000,A=1.000000)" 1e+02)
  (Game|SpawnActorfromClass (Utilities|GetClass (Variables|Default|GetEnemies)) (Math|Transform|MakeTransform (+ (Transformation|GetActorLocation _asbp_iron_soul) (* (Math|Vector|MakeVector (.x _returnvalue) (.y _returnvalue) 0.0) (Math|Random|RandomFloatinRange (Variables|Spawner|GetMin%20Distance) (Variables|Spawner|GetMax%20Distance)))) "0, 0, 0" "1.000000,1.000000,1.000000") "Undefined" "MultiplyWithRoot" 0 0))