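; BP_IronSoul is a player Blueprint that shoots bullets, takes damage and turns to face a target point.
; Fire spawns the current bullet at ShootArrow, targets a found BP_Enemy and binds impact to send damage using the bullet's Attack.
; BPCDamageSystem handles health, healing and damage through wrapper functions.
; Its events, bound in the construction script, enable mesh physics without collision on death and print block and damage responses.
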(event Custom|DamageResponse
  (params (DamageResponse :type Enum_DamageResponse%20Enum :default "NewEnumerator0"))
  ;[1 1 1] Damage System
  (Development|PrintString (Utilities|String|EnumtoString DamageResponse)))

(event Custom|Death
  (bind _mesh (Variables|Character|GetMesh))
  ;[1 1 1] Damage System
  (Physics|SetSimulatePhysics _mesh true)
  (Collision|SetCollisionEnabled _mesh "NoCollision"))

(event Custom|Blocked
  (params (CanBeParried :type Boolean))
  ;[1 1 1] Damage System
  (Development|PrintString "Blocked"))

(event Custom|Fire
  ;[1 1 1] Shoot
  (bind _returnvalue (Actor|GetActorOfClass "/Game/Blueprints/Enemy/BP_Enemy.BP_Enemy_C"))
  (bind _returnvalue_2 (Game|SpawnActorfromClass (Variables|Default|GetCurrentBullet) (Transformation|GetWorldTransform (Variables|Components|GetShootArrow)) "AlwaysSpawn" "MultiplyWithRoot" self 0.0 2e+03 1e+01 1.0 _returnvalue 0))
  (EventDispatchers|BindEventtoImpact _returnvalue_2 (delegate Custom|DamageEnemy)))

(event Custom|DamageEnemy
  (params (Other%20Actor :type Actor%20Object%20Reference) (Hit%20Results :type Hit%20Result%20Structure))
  ;[1 1 1] Shoot
  (Class|BPIDamagable|TakeDamage(Message) Other%20Actor (Utilities|Struct|MakeSTR_DamageInfo (Variables|/Game/Blueprints/Projectile/BP_Bullet.BP_Bullet_C|GetAttack (stale Custom|Fire _returnvalue_2)) "NewEnumerator0")))

(event EventLookat
  (params (Target :type Vector :default "0, 0, 0"))
  (bind _returnvalue (Transformation|GetActorLocation))
  ;[1 1 1] Rotate Player
  (Transformation|SetActorRotation (Math|Rotator|FindLookatRotation (Math|Vector|MakeVector (.x _returnvalue) (.y _returnvalue) 0.0) (Math|Vector|MakeVector (.x Target) (.y Target) 0.0))))

(fn ConstructionScript
  (bind _bpc_damagesystem (Variables|Components|GetBPC_DamageSystem))
  (EventDispatchers|BindEventtoOnDeath _bpc_damagesystem (EventDispatchers|CreateEvent :!event Custom|Death))
  (EventDispatchers|BindEventtoOnBlocked _bpc_damagesystem (EventDispatchers|CreateEvent :!event Custom|Blocked))
  (EventDispatchers|BindEventtoOnDamageResponse _bpc_damagesystem (EventDispatchers|CreateEvent :!event Custom|DamageResponse)))

(fn GetCurrentHealth
  (return (Variables|/Game/Blueprints/Interface/BPC_DamageSystem.BPC_DamageSystem_C|GetHealth (Variables|Components|GetBPC_DamageSystem))))

(fn GetMaxHealth
  (return (Variables|/Game/Blueprints/Interface/BPC_DamageSystem.BPC_DamageSystem_C|GetMaxHealth (Variables|Components|GetBPC_DamageSystem))))

(fn Heal
  (params (Amount :type Float%20%28double-precision%29))
  (bind _new_health (Default|Heal (Variables|Components|GetBPC_DamageSystem) Amount))
  (return _new_health))

(fn TakeDamage
  (params (DamageInfo :type STR%20Damage%20Info%20Structure))
  (bind _was_damaged (Default|TakeDamage (Variables|Components|GetBPC_DamageSystem) DamageInfo))
  (return _was_damaged))