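; BP_BulletShotgun is a shotgun projectile actor that turns one shot into a spread of BP_Bullet actors.
; On BeginPlay it loops over the Shells count, spawning each bullet at its own location with a random direction inside a cone around the Arrow component's forward vector.
; The Angle variable sets the cone half-angle, and each iteration also prints a leftover debug "Hello" string.
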(event EventBeginPlay
  (for _index (range 0 (Variables|Default|GetShells))
    (Development|PrintString "Hello")
    (Game|SpawnActorfromClass "/Game/Blueprints/Projectile/BP_Bullet.BP_Bullet_C" (Math|Transform|MakeTransform (Transformation|GetActorLocation) (Math|Rotator|MakeRotfromX (Math|Random|RandomUnitVectorinConeinDegrees (Math|Vector|GetForwardVector (Variables|Default|GetArrow)) (Variables|Default|GetAngle)))) "Undefined" "MultiplyWithRoot" 0 0.0 2e+03 3.0 1.0 0)))

(fn ConstructionScript
  (|CallParentFunction))