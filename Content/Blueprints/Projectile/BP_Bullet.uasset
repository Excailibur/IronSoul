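; BP_Bullet is a projectile that can optionally home on a target and triggers impact handling when it hits something.
; Construction applies speed, lifetime and homing; BeginPlay ignores the owner and aims homing shots at their target.
; A separate event, not called here, picks the nearest BP_Enemy as homing target.
; Hits on anything but the player character call impact, play effects and sound, then destroy the bullet.
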(event OnComponentHit(Bullet)
  (params (HitComponent :type Primitive%20Component%20Object%20Reference) (OtherActor :type Actor%20Object%20Reference) (OtherComp :type Primitive%20Component%20Object%20Reference) (NormalImpulse :type Vector :default "0, 0, 0") (Hit :type Hit%20Result%20Structure%20%28by%20ref%29))
  (bind _location (Collision|BreakHitResult Hit))
  ;[1 1 1] Bullet Spawner
  (if (not (== OtherActor (Game|GetPlayerCharacter 0)))
    (Default|CallImpact OtherActor Hit)
    (Effects|SpawnEmitteratLocation (Variables|Effects|GetImpact%20Effects) _location)
    (Audio|PlaySoundatLocation (Variables|Sound|GetSound) _location "0, 0, 0" 1.0 1.0 0.0 0 0 0 0)
    (Actor|DestroyActor)))

(event Custom|RotateToTarget
  ;[1 1 1] Rotate Bullet towards Enemy
  (Variables|/Script/Engine.MovementComponent|SetVelocity (Variables|Default|GetProjectileMovement) (* (Math|Vector|GetUnitDirection(Vector) (Transformation|GetActorLocation) (Transformation|GetActorLocation (Variables|Target|GetTarget))) (Variables|PojectileSettings|GetSpeed))))

(event Custom|Find%20Nearest%20Taregt
  ;[1 1 1] Find Nearest Actor
  (bind _outactors (Actor|GetAllActorsOfClass "/Game/Blueprints/Enemy/BP_Enemy.BP_Enemy_C"))
  (bind _output_get (Variables|Target|SetTarget (.ReturnValue (Actor|FindNearestActor (Transformation|GetActorLocation) _outactors))))
  (Variables|/Script/Engine.ProjectileMovementComponent|SetHomingTargetComponent (Variables|Default|GetProjectileMovement) (Variables|/Script/Engine.Actor|GetRootComponent _output_get)))

(event EventBeginPlay
  (Collision|IgnoreActorwhenMoving (Variables|Default|GetBullet) (Components|GetOwner) true)
  (if (Variables|PojectileSettings|GetIsHoming)
    (Variables|Target|GetTarget
      (:then
        (CallFunction|RotatetoTarget))
      (:else))))

(fn ConstructionScript
  (bind _projectilemovement (Variables|Default|GetProjectileMovement))
  (bind _speed (Variables|PojectileSettings|GetSpeed))
  (Variables|/Script/Engine.ProjectileMovementComponent|SetInitialSpeed _projectilemovement _speed)
  (Variables|/Script/Engine.ProjectileMovementComponent|SetMaxSpeed _projectilemovement _speed)
  (Actor|SetLifeSpan (Variables|PojectileSettings|GetLifeTime))
  (Variables|Target|GetTarget
    (:then
      (if (Variables|PojectileSettings|GetIsHoming)
        (Variables|/Script/Engine.ProjectileMovementComponent|SetbIsHomingProjectile _projectilemovement true)))
    (:else)))