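; Game state for the Iron Soul mode that runs the match countdown, flagging game over and a win when time runs out.
; A Delay on Tick paces the countdown to roughly one-second steps, and GetTime formats it as minutes and seconds.
; Each step, RaiseDiffculty passes the BP_EnemySpawner found at BeginPlay a spawn-rate value that shrinks over the last four minute marks.
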(event EventTick
  (params (DeltaSeconds :type Float%20%28single-precision%29))
  (Utilities|FlowControl|Delay 1.0)
  (CallFunction|RaiseDiffculty (Variables|Timer|GetMinute))
  (if (== (Variables|Timer|GetSeconds) 0)
    (if (== (Variables|Timer|GetMinute) 0)
      (if (== (Variables|Timer|GetSeconds) 0)
        (Variables|Default|SetGameOver true)
        (Variables|Default|SetWin true))
      (else
        (Variables|Timer|SetSeconds 59)
        (Variables|Timer|SetMinute (- (Variables|Timer|GetMinute) 1))))
    (else
      (Variables|Timer|SetSeconds (- (Variables|Timer|GetSeconds) 1)))))

(event EventBeginPlay
  (bind _returnvalue (Actor|GetActorOfClass "/Game/Blueprints/Enemy/BP_EnemySpawner.BP_EnemySpawner_C"))
  (Variables|Default|SetEnemySpawner _returnvalue))

(fn ConstructionScript)

(fn GetTime
  (return (Utilities|Text|FormatText "{Minutes} : {Seconds}" (Utilities|Text|ToText(Integer) (Variables|Timer|GetMinute) false true 2) (Utilities|Text|ToText(Integer) (Variables|Timer|GetSeconds) false true 2))))

(fn RaiseDiffculty
  (params (Minute :type Integer))
  (bind _enemyspawner (Variables|Default|GetEnemySpawner))
  (switch int Minute
    (:1
      (Default|UpdateSpawnRate _enemyspawner 0.2))
    (:2
      (Default|UpdateSpawnRate _enemyspawner 0.8))
    (:3
      (Default|UpdateSpawnRate _enemyspawner 1.2))
    (:4
      (Default|UpdateSpawnRate _enemyspawner 1.5))))