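; BP_Bullet is a projectile actor that flies at a set speed and reports what it hits.
; On BeginPlay it applies Speed to the ProjectileMovement component as both initial and maximum speed, and limits its lifespan to LifeTime.
; When the Bullet component hits something, it calls Impact with the other actor and hit result, then destroys itself, leaving the hit response outside this graph.
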(event OnComponentHit(Bullet)
  (params (HitComponent :type Primitive%20Component%20Object%20Reference) (OtherActor :type Actor%20Object%20Reference) (OtherComp :type Primitive%20Component%20Object%20Reference) (NormalImpulse :type Vector :default "0, 0, 0") (Hit :type Hit%20Result%20Structure%20%28by%20ref%29))
  (Default|CallImpact OtherActor Hit)
  (Actor|DestroyActor))

(event EventBeginPlay
  (Variables|/Script/Engine.ProjectileMovementComponent|SetInitialSpeed (Variables|Default|GetProjectileMovement) (Variables|PojectileSettings|GetSpeed))
  (Variables|/Script/Engine.ProjectileMovementComponent|SetMaxSpeed (Variables|Default|GetProjectileMovement) (Variables|PojectileSettings|GetSpeed))
  (Actor|SetLifeSpan (Variables|Default|GetLifeTime)))

(fn ConstructionScript)